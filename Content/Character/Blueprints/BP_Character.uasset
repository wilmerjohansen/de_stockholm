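; First-person player character with Enhanced Input movement, pogo and bunnyhop console settings, crouch-dependent braking friction, and weapon handling.
; Interact messages an overlapping pickup; SpawnWeapon tosses the current weapon as a physics pickup, spawns its replacement and plays draw-to-idle animations.
; CanFire gates firing, with semi and full auto sharing one path.
; Jump and landing play sounds; the sphere-traced footstep check sits on a timeline track marked never run.
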(event `self.ReceiveTick`
  (params (DeltaSeconds :type "Float (single-precision)")))

(event `self.ReceiveBeginPlay`
  (bind _asplayer_controller (cast `PlayerController` (`self.GetController`)))
  (bind _returnvalue (pcsubsystem `EnhancedInputLocalPlayerSubsystem` _asplayer_controller))
  (`/Engine/EditorBlueprintResources/StandardMacros.IsValid` _returnvalue
    (:`Is Valid`
      (`EnhancedInputSubsystemInterface.AddMappingContext` _returnvalue "/Game/Character/Input/IMC_Character.IMC_Character" 0 (struct))
      (`KismetSystemLibrary.ExecuteConsoleCommand` "move.Pogo 1" null)
      (`KismetSystemLibrary.ExecuteConsoleCommand` "move.Bunnyhopping 1" null)
      (`KismetSystemLibrary.ExecuteConsoleCommand` "move.JumpBoost 0" null)
      (`KismetSystemLibrary.ExecuteConsoleCommand` "r.screenpercentage 50" null))))

(event `EnhancedInput|/Game/Character/Input/IA_MoveForward`
  (params (ActionValue :type "Float (double-precision)") (ElapsedSeconds :type "Float (double-precision)") (TriggeredSeconds :type "Float (double-precision)") (InputAction :type "InputAction Object Reference" :default "/Game/Character/Input/IA_MoveForward.IA_MoveForward"))
  (bind _footsteps_tl (`self.Footsteps_TL`))
  (:`Triggered`
    (`self.AddMovementInput` (`GameplayStatics.GetPlayerCharacter` 0) (`self.GetActorForwardVector`) ActionValue false)
    (`TimelineComponent.Play` _footsteps_tl :!label _label))
  (:`Completed`
    (`TimelineComponent.Stop` _footsteps_tl :!label _label_2)))

(event `EnhancedInput|/Game/Character/Input/IA_MoveRight`
  (params (ActionValue :type "Float (double-precision)") (ElapsedSeconds :type "Float (double-precision)") (TriggeredSeconds :type "Float (double-precision)") (InputAction :type "InputAction Object Reference" :default "/Game/Character/Input/IA_MoveRight.IA_MoveRight"))
  (:`Triggered`
    (`self.AddMovementInput` (`GameplayStatics.GetPlayerCharacter` 0) (`self.GetActorRightVector`) ActionValue false)
    (goto _label))
  (:`Completed`
    (goto _label_2)))

(event `EnhancedInput|/Game/Character/Input/IA_Look`
  (params (ActionValue :type "Vector2D Structure") (ElapsedSeconds :type "Float (double-precision)") (TriggeredSeconds :type "Float (double-precision)") (InputAction :type "InputAction Object Reference" :default "/Game/Character/Input/IA_Look.IA_Look"))
  (bind (_x _y) (`KismetMathLibrary.BreakVector2D` ActionValue))
  (bind _returnvalue (`GameplayStatics.GetPlayerCharacter` 0))
  (:`Triggered`
    (`self.AddControllerYawInput` _returnvalue _x)
    (bind _result (`/Engine/EditorBlueprintResources/StandardMacros.NegateFloat` _y)
      (:`  `
        (`self.AddControllerPitchInput` _returnvalue _result)))))

(event `EnhancedInput|/Game/Character/Input/IA_Jump`
  (params (ActionValue :type Boolean) (ElapsedSeconds :type "Float (double-precision)") (TriggeredSeconds :type "Float (double-precision)") (InputAction :type "InputAction Object Reference" :default "/Game/Character/Input/IA_Jump.IA_Jump"))
  (bind _returnvalue (`GameplayStatics.GetPlayerCharacter` 0))
  (:`Triggered`
    (`self.Jump` _returnvalue)
    (if (not (`self.In Air?`))
      (`GameplayStatics.PlaySoundAtLocation` "/Game/Sounds/Misc/jump_launch_01.jump_launch_01" (`self.K2_GetActorLocation`) (struct) 1.0 1.0 0.0 null null null null)
      (set `self.In Air?` true)))
  (:`Canceled`
    (`self.StopJumping` _returnvalue :!label _label_3))
  (:`Completed`
    (goto _label_3)))

(event `EnhancedInput|/Game/Character/Input/IA_Crouch`
  (params (ActionValue :type Boolean) (ElapsedSeconds :type "Float (double-precision)") (TriggeredSeconds :type "Float (double-precision)") (InputAction :type "InputAction Object Reference" :default "/Game/Character/Input/IA_Crouch.IA_Crouch"))
  (bind _returnvalue (`GameplayStatics.GetPlayerCharacter` 0))
  (bind _charactermovement (`self.CharacterMovement`))
  (:`Triggered`
    (if ActionValue
      (`self.Crouch` _returnvalue)
      (set `CharacterMovementComponent.bUseSeparateBrakingFriction` false _charactermovement)
      (else
        (`self.UnCrouch` _returnvalue)
        (set `CharacterMovementComponent.bUseSeparateBrakingFriction` true _charactermovement)))))

(event `self.OnLanded`
  (params (Hit :type "HitResult Structure (by ref)"))
  (`GameplayStatics.PlaySoundAtLocation` "/Game/Sounds/Landing/Tile/TileLandingQue.TileLandingQue" (`self.K2_GetActorLocation`) (struct) 1.0 1.0 0.0 null null null null)
  (set `self.In Air?` false))

(event `EnhancedInput|/Game/Character/Input/IA_Interact`
  (params (ActionValue :type Boolean) (ElapsedSeconds :type "Float (double-precision)") (TriggeredSeconds :type "Float (double-precision)") (InputAction :type "InputAction Object Reference" :default "/Game/Character/Input/IA_Interact.IA_Interact"))
  (:`Triggered`
    (message `/Game/Interfaces/BPI_Interact.Interact` (`|GetArrayItem` (`self.GetOverlappingActors` "/Game/Props/Pickups/BP_PickupMaster.BP_PickupMaster_C")) self)))

(event `Spawn Weapon`
  (params (`Weapon To Spawn` :type "/Game/Weapons/BP_WeaponMaster Class Reference") (`Weapon Skeletal Mesh` :type "SkeletalMesh Object Reference") (`Weapon Draw Anim Montage` :type "AnimMontage Object Reference") (`Weapon Idle Anim Montage` :type "AnimMontage Object Reference"))
  (bind _current_weapon (`self.Current Weapon`))
  (bind _weaponslot (`self.WeaponSlot`))
  (bind _returnvalue (`PlayerCameraManager.GetCameraRotation` (`GameplayStatics.GetPlayerCameraManager` 0)))
  (`/Engine/EditorBlueprintResources/StandardMacros.IsValid` _current_weapon
    (:`Is Valid`
      (set `self.Can Fire?` false)
      (bind _returnvalue_2 (`|SpawnActorFromClass` (`/Game/Weapons/BP_WeaponMaster.Pickup Class` _current_weapon) (`KismetMathLibrary.MakeTransform` (+ (`self.K2_GetActorLocation`) (0.0 0.0 40.0)) (`KismetMathLibrary.Conv_VectorToRotator` (+ (* _returnvalue (1.0 1.0 0.0)) (0.0 0.0 -10.0)))) "Undefined" "MultiplyWithRoot" null null))
      (`PrimitiveComponent.SetPhysicsLinearVelocity` (`/Game/Props/Pickups/BP_PickupMaster.PickupObject` _returnvalue_2) (+ (* _returnvalue (300.0 300.0 0.0)) (0.0 0.0 50.0) (`self.GetVelocity`)) false "None")
      (`self.K2_DestroyActor` _current_weapon))
    (:`Is Not Valid`
      _))
  (bind _returnvalue_3 (`|SpawnActorFromClass` `Weapon To Spawn` (`KismetMathLibrary.MakeTransform` (0.0 0.0 0.0) (struct) (0.0 0.0 0.0)) "Undefined" "MultiplyWithRoot" null null))
  (set `self.Current Weapon` _returnvalue_3)
  (`SkeletalMeshComponent.SetSkeletalMeshAsset` _weaponslot `Weapon Skeletal Mesh`)
  (`SkeletalMeshComponent.SetAnimationMode` _weaponslot "AnimationSingleNode" false)
  (`SkeletalMeshComponent.PlayAnimation` _weaponslot `Weapon Draw Anim Montage` false)
  (`KismetSystemLibrary.RetriggerableDelay` (`AnimationAsset.GetPlayLength` `Weapon Draw Anim Montage`))
  (`SkeletalMeshComponent.PlayAnimation` _weaponslot `Weapon Idle Anim Montage` true)
  (set `self.Can Fire?` true))

(event `EnhancedInput|/Game/Character/Input/IA_Fire`
  (params (ActionValue :type Boolean) (ElapsedSeconds :type "Float (double-precision)") (TriggeredSeconds :type "Float (double-precision)") (InputAction :type "InputAction Object Reference" :default "/Game/Character/Input/IA_Fire.IA_Fire"))
  (bind _current_weapon (`self.Current Weapon`))
  (bind _fire_anim_montage (`/Game/Weapons/BP_WeaponMaster.Fire Anim Montage` _current_weapon))
  (:`Triggered`
    (if (`self.Can Fire?`)
      (set `self.Can Fire?` false)
      (`/Engine/EditorBlueprintResources/StandardMacros.IsValid` _current_weapon
        (:`Is Valid`
          (switch `/Game/Weapons/Enum_FireMode` (`/Game/Weapons/BP_WeaponMaster.Fire Mode` _current_weapon)
            (:`NewEnumerator0`
              _)
            (:`NewEnumerator2`
              _))
          (message `/Game/Interfaces/BPI_Fire.Fire` _current_weapon)
          (`SkeletalMeshComponent.PlayAnimation` (`self.WeaponSlot`) _fire_anim_montage false)
          (`KismetSystemLibrary.RetriggerableDelay` 0.0)
          (set `self.Can Fire?` true)
          (`KismetSystemLibrary.RetriggerableDelay` (- (`AnimationAsset.GetPlayLength` _fire_anim_montage) 0.0))
          (if (`self.Can Fire?`)
            (`SkeletalMeshComponent.PlayAnimation` (`self.WeaponSlot`) (`/Game/Weapons/BP_WeaponMaster.Idle Anim Montage` (`self.Current Weapon`)) true)))))))

(fn `FootstepTry`
  (bind _finished (`self.TraceFootsteps`))
  (if _finished
    (`GameplayStatics.PlaySoundAtLocation` "/Game/Sounds/Footsteps/Concrete/ConcreteFootstepsCue.ConcreteFootstepsCue" (`self.K2_GetActorLocation`) (struct) 1.0 1.0 0.0 null null null null)))

(fn `TraceFootsteps`
  (returns (Finished :type Boolean))
  (bind _returnvalue (`self.K2_GetActorLocation`))
  (bind _capsulecomponent (`self.CapsuleComponent`))
  (bind (_outhits _returnvalue_2) (`KismetSystemLibrary.SphereTraceMulti` _returnvalue (`KismetMathLibrary.MakeVector` (.x _returnvalue) (.y _returnvalue) (- (.z _returnvalue) (`CapsuleComponent.GetScaledCapsuleHalfHeight` _capsulecomponent))) (`CapsuleComponent.GetScaledCapsuleRadius` _capsulecomponent) "TraceTypeQuery1"))
  (return _returnvalue_2))

(fn `UserConstructionScript`)