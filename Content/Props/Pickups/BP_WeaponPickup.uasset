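; BP_WeaponPickup is a weapon pickup prop that gives its weapon to the character that interacts with it.
; On Interact, it passes its weapon to spawn, skeletal mesh, and draw and idle montages to that character's SpawnWeapon, then destroys itself.
; The character handles the actual spawning, so the pickup only carries the weapon data and has no active tick or overlap logic.
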(event `/Game/Interfaces/BPI_Interact.Interact`
  (params (CharacterPickinngUp :type "/Game/Character/Blueprints/BP_Character Object Reference"))
  (`/Game/Character/Blueprints/BP_Character.Spawn Weapon` CharacterPickinngUp (`self.Weapon To Spawn`) (`self.Weapon Skeletal Mesh`) (`self.Weapon Draw Anim Montage`) (`self.Weapon Idle Anim Montage`))
  (`self.K2_DestroyActor`))

(fn `UserConstructionScript`
  (`parent.UserConstructionScript`))